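; Menhir actor that holds the village's life pool and triggers the player's defeat when it runs out.
; On BeginPlay it fills life to the maximum, caches the ThirdPersonCharacter and starts a Delay loop that keeps the runes mesh slowly spinning.
; ChangeVillageLife applies a clamped change and calls Defeated on the cached character once life hits zero.
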(event `Rotate Runes`
  (`SceneComponent.K2_AddLocalRotation` (`self.RunesMesh`) (struct :`Yaw` 0.1) false false :!label _label)
  (`KismetSystemLibrary.Delay` 0.02)
  (goto _label))

(event `self.ReceiveBeginPlay`
  (set `self.VillageLife` (`self.Max VIllage Life`))
  (bind _asthird_person_character (cast `/Game/ThirdPersonBP/Blueprints/ThirdPersonCharacter` (`GameplayStatics.GetPlayerCharacter` 0)))
  (set `self.Player Character` _asthird_person_character)
  (`self.Rotate Runes`))

(event `Change Village Life`
  (params (`Life Change` :type "Float (double-precision)"))
  (bind _output_get (set `self.VillageLife` (`KismetMathLibrary.FClamp` (+ (`self.VillageLife`) `Life Change`) 0.0 (`self.Max VIllage Life`))))
  (`/Engine/EditorBlueprintResources/StandardMacros.CompareFloat` _output_get
    (:`==`
      (`/Game/ThirdPersonBP/Blueprints/ThirdPersonCharacter.Defeated` (`self.Player Character`)))))

(fn `UserConstructionScript`)