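; Village gate Blueprint with two doors that swing open or closed on Interact while the third-person character is inside the trigger volume.
; Overlap events on OpenDoorCollision set CanOpen, and a FlipFlop alternates between opening and closing.
; Each direction rotates both doors oppositely in a Delay loop until the left door's yaw reaches its limit.
; Stop flags let a new interaction interrupt the running swing and reverse it.
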(event `Interact`
  (bind _gatedoor_l (`self.GateDoor_L`))
  (bind _gatedoor_l_2 (`self.GateDoor_L`))
  (if (`self.Can Open`)
    (set `self.StopOpening` false)
    (set `self.StopClosing` false)
    (`/Engine/EditorBlueprintResources/StandardMacros.FlipFlop`
      (:`A`
        (set `self.StopClosing` true)
        (if (not (`self.StopOpening`)) :!label _label
          (`SceneComponent.K2_AddLocalRotation` _gatedoor_l_2 (struct :`Yaw` -2.0) false false)
          (`SceneComponent.K2_AddLocalRotation` (`self.GateDoor_R`) (struct :`Yaw` 2.0) false false)
          (`KismetSystemLibrary.Delay` 0.01)
          (`/Engine/EditorBlueprintResources/StandardMacros.CompareFloat` (.yaw (`SceneComponent.RelativeRotation` _gatedoor_l_2)) -90.0
            (:`>`
              (goto _label)))))
      (:`B`
        (set `self.StopOpening` true)
        (if (not (`self.StopClosing`)) :!label _label_2
          (`SceneComponent.K2_AddLocalRotation` _gatedoor_l (struct :`Yaw` 2.0) false false)
          (`SceneComponent.K2_AddLocalRotation` (`self.GateDoor_R`) (struct :`Yaw` -2.0) false false)
          (`KismetSystemLibrary.Delay` 0.01)
          (`/Engine/EditorBlueprintResources/StandardMacros.CompareFloat` (.yaw (`SceneComponent.RelativeRotation` _gatedoor_l))
            (:`<`
              (goto _label_2))))))))

(event `self.OpenDoorCollision.OnComponentBeginOverlap`
  (params (OverlappedComponent :type "PrimitiveComponent Object Reference") (OtherActor :type "Actor Object Reference") (OtherComp :type "PrimitiveComponent Object Reference") (OtherBodyIndex :type Integer) (bFromSweep :type Boolean) (SweepResult :type "HitResult Structure (by ref)"))
  (cast `/Game/ThirdPersonBP/Blueprints/ThirdPersonCharacter` OtherActor)
  (set `self.Can Open` true))

(event `self.OpenDoorCollision.OnComponentEndOverlap`
  (params (OverlappedComponent :type "PrimitiveComponent Object Reference") (OtherActor :type "Actor Object Reference") (OtherComp :type "PrimitiveComponent Object Reference") (OtherBodyIndex :type Integer))
  (cast `/Game/ThirdPersonBP/Blueprints/ThirdPersonCharacter` OtherActor)
  (set `self.Can Open` false))

(fn `UserConstructionScript`)