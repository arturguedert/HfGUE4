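; Actor component that gives its owner's skeletal mesh physical-animation hit reactions and ragdoll, and applies combat damage between the player and enemies.
; BeginPlay creates the physical animation component; hits simulate bodies below Spine1, while Tick fades blend weight and then stops simulation.
; Torso or head hits add an impulse and deal the attacker's damage; left forearm hits only print "Blocked".
; Ragdoll simulates from Root with its own profile.
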(event `self.ReceiveBeginPlay`
  (bind _returnvalue (`self.GetOwner`))
  (bind _returnvalue_2 (`Actor.GetComponentByClass` _returnvalue "/Script/Engine.SkeletalMeshComponent"))
  (bind _returnvalue_3 (`|AddComponentByClass` _returnvalue "/Script/Engine.PhysicalAnimationComponent"))
  (bind _output_get (set `self.Physical Animation Component` _returnvalue_3))
  (`PhysicalAnimationComponent.SetSkeletalMeshComponent` _output_get _returnvalue_2)
  (set `self.Skeletal Mesh` _returnvalue_2))

(event `Toggle Physical Animation`
  (params (`SimON?` :type Boolean :default true))
  (`self.Enable Physical Animation` (`self.Skeletal Mesh`) (`self.Physical Animation Component`)))

(event `Enter Ragdoll`
  (`SkeletalMeshComponent.SetAllBodiesBelowSimulatePhysics` (`self.Skeletal Mesh`) "Root" true true)
  (`PhysicalAnimationComponent.ApplyPhysicalAnimationProfileBelow` (`self.Physical Animation Component`) "Root" "Ragdoll" false false))

(event `Hit Reaction`
  (params (Hit :type "HitResult Structure") (HitStrength :type "Float (double-precision)" :default 5000.0) (Attacker :type "Actor Object Reference"))
  (bind (_bblockinghit _binitialoverlap _time _distance _location _impactpoint _normal _impactnormal _physmat _hitactor _hitcomponent _hitbonename _hititem _elementindex _faceindex _tracestart _traceend) (`GameplayStatics.BreakHitResult` Hit))
  (bind _returnvalue (select `bool` (== _hitbonename "Root") :`false` _hitbonename :`true` "Spine1"))
  (set `self.Attacker` Attacker)
  (`self.SetComponentTickEnabled` true)
  (`self.Enable Physical Animation` (`self.Skeletal Mesh`) (`self.Physical Animation Component`))
  (set `self.Hit Reaction Time Remaining` (+ (`self.Hit Reaction Time Remaining`) 2.0))
  (if (== _hitbonename "LowerArm_L")
    (`KismetSystemLibrary.PrintString` "Blocked")
    (elif (or (== _returnvalue "Spine1") (== _returnvalue "Spine2") (== _returnvalue "Head"))
      (`PrimitiveComponent.AddImpulse` (`self.Skeletal Mesh`) (* (`KismetMathLibrary.Normal` (- _traceend _tracestart)) HitStrength) _returnvalue true)
      (`|ExecutionSequence`
        (:`then_0`
          (bind _asenemy_bp (cast `/Game/Characters/Soldado/Enemy_BP` (`self.GetOwner`)))
          (bind _asthird_person_character (cast `/Game/ThirdPersonBP/Blueprints/ThirdPersonCharacter` (`self.Attacker`)))
          (`/Game/Characters/Soldado/Enemy_BP.Take Damage` _asenemy_bp (`/Game/ThirdPersonBP/Blueprints/ThirdPersonCharacter.Attack Damage` _asthird_person_character)))
        (:`then_1`
          (bind _asthird_person_character_2 (cast `/Game/ThirdPersonBP/Blueprints/ThirdPersonCharacter` (`self.GetOwner`)))
          (bind _asenemy_bp_2 (cast `/Game/Characters/Soldado/Enemy_BP` (`self.Attacker`)))
          (`/Game/ThirdPersonBP/Blueprints/ThirdPersonCharacter.Change Life` _asthird_person_character_2 (`/Game/Characters/Soldado/Enemy_BP.Attack Damage` _asenemy_bp_2)))))))

(event `self.ReceiveTick`
  (params (DeltaSeconds :type "Float (single-precision)"))
  (set `self.Hit Reaction Time Remaining` (- (`KismetMathLibrary.FInterpTo` (`self.Hit Reaction Time Remaining`) 0.0 0.0 5.0) (* DeltaSeconds 5.0)))
  (if (<= (`self.Hit Reaction Time Remaining`) 0.0)
    (set `self.Hit Reaction Time Remaining` 0.0)
    (`SkeletalMeshComponent.SetAllBodiesBelowSimulatePhysics` (`self.Skeletal Mesh`) "Spine1" false true)
    (`self.SetComponentTickEnabled` false)
    (else
      (`SkeletalMeshComponent.SetAllBodiesBelowPhysicsBlendWeight` (`self.Skeletal Mesh`) "Spine1" (`KismetMathLibrary.FMin` (`self.Hit Reaction Time Remaining`) 1.0) false true))))

(fn `Enable Physical Animation`
  (params (Mesh :type "PrimitiveComponent Object Reference") (`Physical Anim Component` :type "PhysicalAnimationComponent Object Reference"))
  (`PrimitiveComponent.SetCollisionEnabled` Mesh "QueryAndPhysics")
  (`SkeletalMeshComponent.SetAllBodiesBelowSimulatePhysics` (`Actor.GetComponentByClass` (`self.GetOwner` Mesh) "/Script/Engine.SkeletalMeshComponent") "Spine1" true true)
  (`PhysicalAnimationComponent.ApplyPhysicalAnimationProfileBelow` `Physical Anim Component` "Spine1" "Strong" true false))