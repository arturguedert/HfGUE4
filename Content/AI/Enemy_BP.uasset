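; Enemy character Blueprint that patrols, searches, chases and attacks the player, and can be punched to death.
; It runs a behavior tree, with PawnSensing sight and noise driving timed state changes shown by a colored indicator.
; Punching hit zones overlapping the capsule apply damage, record hit direction and trigger chase.
; Death ragdolls the mesh with an impulse scaled by the player's punch and damage, then destroys the actor.
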(event `self.ReceiveBeginPlay`
  (bind _returnvalue (`AIBlueprintHelperLibrary.GetAIController` self))
  (`|ExecutionSequence`
    (:`then_0`
      ;[1 1 1] Setup
      (bind _returnvalue_2 (`GameplayStatics.GetActorOfClass` "/Game/BluePrints/Menhir_BP.Menhir_BP_C"))
      (set `self.Menhir` _returnvalue_2)
      (bind _returnvalue_3 (`GameplayStatics.GetActorOfClass` "/Game/ThirdPersonBP/Blueprints/ThirdPersonCharacter.ThirdPersonCharacter_C"))
      (set `self.Player` _returnvalue_3)
      (set `self.Current Life` (`self.Max Life`)))
    (:`then_1`
      (if (!= _returnvalue null)
        (`AIController.UseBlackboard` _returnvalue "/Game/AI/EnemyBlackBoard.EnemyBlackBoard")
        (`AIController.RunBehaviorTree` _returnvalue "/Game/AI/EnemyAI_BT.EnemyAI_BT")))
    (:`then_2`
      (bind _outactors (`GameplayStatics.GetAllActorsOfClass` "/Script/Engine.TargetPoint"))
      (set `self.Target Points` _outactors))))

(event `self.ReceiveTick`
  (params (DeltaSeconds :type "Float (single-precision)")))

(event `self.CapsuleComponent.OnComponentBeginOverlap`
  (params (OverlappedComponent :type "PrimitiveComponent Object Reference") (OtherActor :type "Actor Object Reference") (OtherComp :type "PrimitiveComponent Object Reference") (OtherBodyIndex :type Integer) (bFromSweep :type Boolean) (SweepResult :type "HitResult Structure (by ref)"))
  (bind _returnvalue (`KismetSystemLibrary.GetObjectName` OtherComp))
  ;[1 1 1] Hit
  (if (or (`KismetStringLibrary.EqualEqual_StrStr` _returnvalue "HitZoneL") (`KismetStringLibrary.EqualEqual_StrStr` _returnvalue "HitZoneR"))
    (bind _asthird_person_character (cast `/Game/ThirdPersonBP/Blueprints/ThirdPersonCharacter` OtherActor))
    (if (`/Game/ThirdPersonBP/Blueprints/ThirdPersonCharacter.Punching` _asthird_person_character)
      (set `self.Hit` true)
      (`/Engine/EditorBlueprintResources/StandardMacros.DoOnce` false :!label _label
        (:`Completed`
          (`self.Take Damage` (`/Game/ThirdPersonBP/Blueprints/ThirdPersonCharacter.Attack Damage` _asthird_person_character))
          (bind (_returnvalue_x _returnvalue_y) (`KismetMathLibrary.BreakVector` (`KismetMathLibrary.Normal` (`KismetMathLibrary.InverseTransformLocation` (`self.GetTransform`) (`self.K2_GetActorLocation` _asthird_person_character)) 0.01)))
          (set `self.HitReactionX` _returnvalue_x)
          (set `self.HitReactionY` _returnvalue_y)
          (`KismetSystemLibrary.Delay` 0.5)
          (set `self.Hit` false)
          (`self.Enter Chase State`)
          (goto _label :!via `Reset`))))))

(event `Attack`
  ;[1 1 1] Attack
  (`/Engine/EditorBlueprintResources/StandardMacros.DoOnce` false :!label _label_2
    (:`Completed`
      (if (not (`self.Attacking`))
        (set `self.AIState` "NewEnumerator3")
        (set `self.Attacking` true)
        (`KismetSystemLibrary.Delay` 0.1)
        (set `self.Attacking` false)
        (`KismetSystemLibrary.Delay` (`self.Attack Cooldown`))
        (goto _label_2 :!via `Reset`)))))

(event `Take Damage`
  (params (Damage :type "Float (double-precision)"))
  ;[1 1 1] Take Damage
  (bind _output_get (set `self.Current Life` (- (`self.Current Life`) Damage)))
  (`KismetSystemLibrary.PrintString` (`KismetStringLibrary.Conv_DoubleToString` _output_get))
  (if (<= _output_get 0.0)
    (`self.Death Sequence`)
    (else
      (`KismetSystemLibrary.Delay` 0.2))))

(event `Death Sequence`
  (bind _player (`self.Player`))
  (bind _mesh (`self.Mesh`))
  (bind (_returnvalue_x _returnvalue_y) (`KismetMathLibrary.BreakVector` (`KismetMathLibrary.GetForwardVector` (`self.K2_GetActorRotation` _player))))
  ;[1 1 1] Death
  (`self.SetActorTickEnabled` false)
  (`KismetSystemLibrary.PrintString` "Enemy Dead")
  (`PrimitiveComponent.SetSimulatePhysics` _mesh true)
  (`PrimitiveComponent.SetCollisionProfileName` _mesh "Ragdoll" true)
  (`PrimitiveComponent.AddImpulse` _mesh (* (`KismetMathLibrary.MakeVector` _returnvalue_x _returnvalue_y (select `int` (`/Game/ThirdPersonBP/Blueprints/ThirdPersonCharacter.Punch Index` _player) :`0` 0.4 :`1` 0.4 :`2` 0.8 :!type "Float (single-precision)")) (* 2000 (`/Game/ThirdPersonBP/Blueprints/ThirdPersonCharacter.Attack Damage` _player))) "Spine2" false)
  (`PrimitiveComponent.SetCollisionEnabled` (`self.CapsuleComponent`) "NoCollision")
  (`KismetSystemLibrary.Delay` 4.0)
  (`self.K2_DestroyActor`))

(event `self.PawnSensing.OnSeePawn`
  (params (Pawn :type "Pawn Object Reference"))
  ;[1 1 1] AI States
  (bind _asthird_person_character (cast `/Game/ThirdPersonBP/Blueprints/ThirdPersonCharacter` Pawn))
  (set `self.Seen Player` _asthird_person_character)
  (`self.Enter Chase State`))

(event `self.PawnSensing.OnHearNoise`
  (params (Instigator :type "Pawn Object Reference") (Location :type "Vector Structure (by ref)") (Volume :type "Float (single-precision)"))
  ;[1 1 1] AI States
  (cast `/Game/ThirdPersonBP/Blueprints/ThirdPersonCharacter` Instigator)
  (bind _output_get (set `self.NoiseLocation` Location))
  (if (not (`|EnumEquality` (`self.AIState`) "NewEnumerator2"))
    (`self.Enter Search State` _output_get)))

(event `Enter Patrol State`
  ;[1 1 1] AI States
  (set `self.AIState` "NewEnumerator0")
  (`self.UpdateStateInd` (struct :`G` 1.0 :`A` 1.0)))

(event `Enter Search State`
  (params (`Noise Location` :type "Vector Structure"))
  ;[1 1 1] AI States
  (set `self.AIState` "NewEnumerator1")
  (`BlackboardComponent.SetValueAsVector` (`AIBlueprintHelperLibrary.GetBlackboard` null) "NextTarget" `Noise Location`)
  (`self.UpdateStateInd` (struct :`R` 1.0 :`G` 1.0 :`A` 1.0))
  (`KismetSystemLibrary.Delay` 5.0)
  (`self.Enter Patrol State`))

(event `Enter Chase State`
  ;[1 1 1] AI States
  (`BlackboardComponent.SetValueAsBool` (`AIBlueprintHelperLibrary.GetBlackboard` null) "PlayerSeen" true)
  (set `self.AIState` "NewEnumerator2")
  (`self.UpdateStateInd` (struct :`R` 1.0 :`A` 1.0))
  (`KismetSystemLibrary.Delay` 5.0)
  (`self.Enter Search State` (`self.K2_GetActorLocation`)))

(event `UpdateStateInd`
  (params (`Ind Color` :type "LinearColor Structure"))
  ;[1 1 1] AI States
  (bind _returnvalue (`PrimitiveComponent.CreateDynamicMaterialInstance` (`self.State Indicator`) 0 "/Game/AI/Materials/StateIndicator_Mat.StateIndicator_Mat" "None"))
  (`MaterialInstanceDynamic.SetVectorParameterValue` _returnvalue "Color" `Ind Color`))

(fn `UserConstructionScript`)